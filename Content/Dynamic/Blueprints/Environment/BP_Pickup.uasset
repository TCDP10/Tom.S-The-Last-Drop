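; BP_Pickup is a physics-simulated pickup actor whose Cube mesh can be picked up by a bubble through an Interact event.
; On BeginPlay it enables physics on the Cube, registers itself with its ACBubblePickUp component and calls that component's GetSelfTransform.
; Interact delegates to the component's Pickup, passing the bubble reference, the Cube, a simulate-physics flag and the BubbleFalloff setting.
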(event `self.ReceiveBeginPlay`
  (bind _ac_bubblepickup (`self.AC_BubblePickUp`))
  (`PrimitiveComponent.SetSimulatePhysics` (`self.Cube`) true)
  (set `/Game/Dynamic/Blueprints/Environment/AC_BubblePickUp.SelfActor` self _ac_bubblepickup)
  (`/Game/Dynamic/Blueprints/Environment/AC_BubblePickUp.GetSelfTransform` _ac_bubblepickup))

(event `/Game/Dynamic/Blueprints/Core/BPI_BubbleInteract.Interact`
  (params (BubbleRef :type "/Game/Dynamic/Blueprints/Characters/BubbleChar/BP_BubbleChar Object Reference"))
  (`/Game/Dynamic/Blueprints/Environment/AC_BubblePickUp.Pickup` (`self.AC_BubblePickUp`) BubbleRef (`self.Cube`) true (`self.Bubble Falloff`)))

(fn `UserConstructionScript`)